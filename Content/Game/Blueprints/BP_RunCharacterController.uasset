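; BP_RunCharacterController drives the player's BP_RunCharacter in auto-run movement, with constant forward motion and player-controlled sideways steering.
; BeginPlay caches the pawn as BP_RunCharacter and adds the IMC_Run Enhanced Input mapping context.
; Tick feeds full forward movement input every frame, while IA_Run's X value adds movement along the pawn's right vector.
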(event Input|EnhancedActionEvents|EnhancedInputActionIA_Run
  (params (ActionValue :type Vector%202D%20Structure) (ElapsedSeconds :type Float%20%28double-precision%29) (TriggeredSeconds :type Float%20%28double-precision%29) (InputAction :type Input%20Action%20Object%20Reference :default "/Game/Game/Input/IA_Run.IA_Run"))
  (Pawn|Input|AddMovementInput (Variables|Default|GetAs%20BP%20Run%20Character) (Transformation|GetActorRightVector (Game|Player|GetPlayerPawn 0)) (.x ActionValue) false))

(event EventTick
  (params (DeltaSeconds :type Float%20%28single-precision%29))
  (Pawn|Input|AddMovementInput (Variables|Default|GetAs%20BP%20Run%20Character) (Transformation|GetActorForwardVector (Game|Player|GetPlayerPawn 0)) 1.0 false))

(event EventBeginPlay
  (bind _returnvalue (Game|GetPlayerController 0))
  (bind _returnvalue_2 (PlayerController|LocalPlayerSubsystems|GetEnhancedInputLocalPlayerSubsystem _returnvalue))
  (bind _asbp_run_character (Utilities|Casting|CastToBP_RunCharacter (Game|Player|GetPlayerPawn 0)))
  (Variables|Default|SetAs%20BP%20Run%20Character _asbp_run_character)
  (Utilities|IsValid _returnvalue_2
    (:Is%20Valid
      (Input|AddMappingContext _returnvalue_2 "/Game/Game/Input/IMC_Run.IMC_Run" 0 "(bIgnoreAllPressedKeysUntilRelease=True,bForceImmediately=False,bNotifyUserSettings=False)"))))

(fn ConstructionScript)