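; Floor tile for an endless-runner style game that randomly populates itself with rock obstacles and coin pickups.
; On BeginPlay it attempts one obstacle and a random number of coins, each chance-gated and added as child actors atop trigger boxes.
; When the run character overlaps EndTrigger, it fires the Exited dispatcher and destroys itself after a short delay.
; GetAttachTransform exposes the AttachPoint's world transform.
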(event OnComponentBeginOverlap(EndTrigger)
  (params (OverlappedComponent :type Primitive%20Component%20Object%20Reference) (OtherActor :type Actor%20Object%20Reference) (OtherComp :type Primitive%20Component%20Object%20Reference) (OtherBodyIndex :type Integer) (bFromSweep :type Boolean) (SweepResult :type Hit%20Result%20Structure%20%28by%20ref%29))
  (Utilities|Casting|CastToBP_RunCharacter OtherActor)
  (Default|CallExited self)
  (Utilities|FlowControl|Delay 0.5)
  (Actor|DestroyActor))

(event EventBeginPlay
  (Variables|Default|SetObstacleSpawnChance 0.6)
  (Variables|Default|SetPickupSpawnChance 0.6)
  (Variables|Default|SetObstacles (Utilities|Array|MakeArray "/Game/Game/Blueprints/BP_RockObstacle.BP_RockObstacle_C" "/Game/Game/Blueprints/BP_RockObstacle1.BP_RockObstacle1_C"))
  (CallFunction|SpawnObstacles (Variables|Default|GetBoxTrigger))
  (Variables|Default|SetPickup (Utilities|Array|MakeArray "/Game/Game/Blueprints/BP_Coin.BP_Coin_C"))
  (for _index (range 0 (Math|Random|RandomInteger 6))
    (CallFunction|SpawnPickup (Variables|Default|GetCoinTrigger))))

(fn ConstructionScript)

(fn GetAttachTransform
  (return (Transformation|GetWorldTransform (Variables|Default|GetAttachPoint))))

(fn RandomPointinBoundingBox
  (params (Box%20Area :type Box%20Component%20Object%20Reference))
  (bind _returnvalue (Components|Box|GetScaledBoxExtent Box%20Area))
  (bind _output_get (LocalVariables|SetRandom%20Position (Math|Vector|MakeVector (Math|Random|RandomFloatinRange (* (.x _returnvalue) -1.0) (.x _returnvalue)) (Math|Random|RandomFloatinRange (* (.y _returnvalue) -1.0) (.y _returnvalue)) (.z _returnvalue))))
  (return _output_get))

(fn SpawnObstacles
  (params (Box%20Area :type Box%20Component%20Object%20Reference))
  (bind _position (CallFunction|RandomPointinBoundingBox Box%20Area))
  (if (< (Math|Random|RandomFloatinRange 0.0 1.0) (Variables|Default|GetObstacleSpawnChance))
    (bind _returnvalue (AddComponent|AddChildActorComponent false (Math|Conversions|ToTransform(Vector) (+ _position (Variables|/Script/Engine.SceneComponent|GetRelativeLocation Box%20Area)))))
    (ChildActorComponent|SetChildActorClass _returnvalue (.OutItem (Utilities|Array|Random (Variables|Default|GetObstacles))))))

(fn SpawnPickup
  (params (Coin%20Area :type Box%20Component%20Object%20Reference))
  (bind _position (CallFunction|RandomPointinBoundingBox Coin%20Area))
  (if (< (Math|Random|RandomFloatinRange 0.0 1.0) (Variables|Default|GetPickupSpawnChance))
    (bind _returnvalue (AddComponent|AddChildActorComponent false (Math|Conversions|ToTransform(Vector) (+ _position (Variables|/Script/Engine.SceneComponent|GetRelativeLocation Coin%20Area)))))
    (ChildActorComponent|SetChildActorClass _returnvalue (.OutItem (Utilities|Array|Random (Variables|Default|GetPickup))))))