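; BP_Pickup is a pickup actor that BP_RunCharacter collects by overlapping its static mesh.
; The overlap casts to BP_RunCharacter and fires OnPlayerOverlap, which checks CanBePickup before calling OnPickup.
; OnPickup plays the Coin sound at the actor's location and destroys it.
; CanBePickup always returns true here, so every character overlap results in a pickup.
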(event OnComponentBeginOverlap(StaticMesh)
  (params (OverlappedComponent :type Primitive%20Component%20Object%20Reference) (OtherActor :type Actor%20Object%20Reference) (OtherComp :type Primitive%20Component%20Object%20Reference) (OtherBodyIndex :type Integer) (bFromSweep :type Boolean) (SweepResult :type Hit%20Result%20Structure%20%28by%20ref%29))
  (bind _asbp_run_character (Utilities|Casting|CastToBP_RunCharacter OtherActor))
  (CallFunction|OnPlayerOverlap _asbp_run_character))

(event Custom|OnPickup
  (params (Character :type BP%20Run%20Character%20Object%20Reference))
  (Audio|PlaySoundatLocation "/Game/Game/SFX/coin.coin" (Transformation|GetActorLocation) "0, 0, 0" 1.0 1.0 0.0 0 0 0 0)
  (Actor|DestroyActor))

(event Custom|OnPlayerOverlap
  (params (Character :type BP%20Run%20Character%20Object%20Reference))
  (bind _canbepickedup (CallFunction|CanbePickup Character))
  (if _canbepickedup
    (CallFunction|OnPickup Character)))

(fn ConstructionScript)

(fn CanbePickup
  (params (Character :type BP%20Run%20Character%20Object%20Reference))
  (return true))