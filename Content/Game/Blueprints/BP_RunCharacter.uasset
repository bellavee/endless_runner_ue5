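; BP_RunCharacter is a character Blueprint whose only scripted logic is a Die event that handles player death.
; Once a cast confirms the player controller is BP_RunCharacterController, it spawns an explosion at the player character, plays a sound at world origin and hides the mesh.
; It then sets the IsDie flag and, after a short delay, restarts the level through a console command.
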(event Custom|Die
  (Utilities|Casting|CastToBP_RunCharacterController (Game|GetPlayerController 0))
  (Effects|SpawnEmitteratLocation "/Game/StarterContent/Particles/P_Explosion.P_Explosion" (Transformation|GetActorLocation (Game|GetPlayerCharacter 0)))
  (Audio|PlaySoundatLocation "/Game/StarterContent/Audio/Explosion01.Explosion01" "0, 0, 0" "0, 0, 0" 1.0 1.0 0.0 0 0 0 0)
  (Rendering|SetVisibility (Variables|Character|GetMesh) false false)
  (Variables|Default|SetIsDie true)
  (Utilities|FlowControl|Delay 3.0)
  (Development|ExecuteConsoleCommand (Variables|Default|GetRestartLevel) 0))

(fn ConstructionScript)