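; BP_RunGameMode is the game mode for a runner level built from chained floor tiles.
; On BeginPlay it shows the WB_RunHUB widget and spawns an initial run of tiles.
; AddFloorTile spawns each BP_FloorTile at the stored attach point, binds its exit event, then advances that point using the tile's attach transform.
; OnTileExited adds another tile to extend the track endlessly, and RestartLevel resets the level.
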(event Custom|Restart%20Level
  (Class|GameModeBase|ResetLevel))

(event Custom|OnTileExited
  (params (Tile :type BP%20Floor%20Tile%20Object%20Reference))
  (CallFunction|AddFloorTile))

(event EventBeginPlay
  (bind _returnvalue (UserInterface|CreateWidget "/Game/Game/UMG/WB_RunHUB.WB_RunHUB_C"))
  (UserInterface|Viewport|AddtoViewport _returnvalue 0)
  (for _index (range 0 2)
    (CallFunction|AddFloorTile)))

(fn ConstructionScript)

(fn AddFloorTile
  (bind _returnvalue (Game|SpawnActorfromClass "/Game/Game/Blueprints/BP_FloorTile.BP_FloorTile_C" (Variables|Default|GetNext%20Attach%20Point) "Undefined" "MultiplyWithRoot" 0 0))
  (EventDispatchers|BindEventtoExited _returnvalue (EventDispatchers|CreateEvent :!event Custom|OnTileExited))
  (bind _attachtransform (Default|GetAttachTransform _returnvalue))
  (Variables|Default|SetNext%20Attach%20Point _attachtransform))